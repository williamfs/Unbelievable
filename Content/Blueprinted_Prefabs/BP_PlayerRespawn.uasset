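; BP_PlayerRespawn is a checkpoint actor that updates where the player respawns.
; On BeginPlay it caches a reference to BP_GameMode.
; When the player pawn overlaps it, it writes its own location to the game mode's PlayerSpawnLoc and prints that value to the screen.
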(event `self.ReceiveBeginPlay`
  ;[1 1 1] Set Refs
  (bind _asbp_game_mode (cast `/Game/Blueprinted_Prefabs/BP_GameMode` (`GameplayStatics.GetGameMode`)))
  (set `self.REFGameMode` _asbp_game_mode))

(event `self.ReceiveActorBeginOverlap`
  (params (OtherActor :type "Actor Object Reference"))
  ;[1 1 1] Setting This Spawn Loc on Overlap
  (if (== OtherActor (`GameplayStatics.GetPlayerPawn` 0))
    (bind _output_get (set `/Game/Blueprinted_Prefabs/BP_GameMode.PlayerSpawnLoc` (`self.K2_GetActorLocation`) (`self.REFGameMode`)))
    (`KismetSystemLibrary.PrintString` (`KismetStringLibrary.Conv_VectorToString` _output_get))))

(fn `UserConstructionScript`)