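; BP_DeathVolume is a kill volume that triggers player death when the player's pawn overlaps it.
; On BeginPlay it caches references to BP_GameMode and BP_GameInstance.
; On overlap it calls PlayerDeath on the game mode, increments NumberOfDeaths on the game instance and prints the total.
; Unconnected leftover nodes hold an older respawn that moved the player to SpawnLocation and reset breaking platforms.
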(event `self.ReceiveBeginPlay`
  ;[1 1 1] Set Refs
  (bind _asbp_game_mode (cast `/Game/Blueprints/BP_GameMode` (`GameplayStatics.GetGameMode`)))
  (set `self.REFGameMode` _asbp_game_mode)
  (bind _asbp_game_instance (cast `/Game/Blueprints/BP_GameInstance` (`GameplayStatics.GetGameInstance`))
    (:`then`
      (set `self.REFGameInstance` _asbp_game_instance))
    (:`CastFailed`
      (`KismetSystemLibrary.PrintString` "No Cast to BP_GameInstance"))))

(event `self.ReceiveActorBeginOverlap`
  (params (OtherActor :type "Actor Object Reference"))
  (bind _refgameinstance (`self.REFGameInstance`))
  ;[1 1 1] Set Player Loc
  (if (== OtherActor (`GameplayStatics.GetPlayerPawn` 0))
    (`/Game/Blueprints/BP_GameMode.PlayerDeath` (`self.REFGameMode`))
    (bind _output_get (set `/Game/Blueprints/BP_GameInstance.NumberOfDeaths` (+ (`/Game/Blueprints/BP_GameInstance.NumberOfDeaths` _refgameinstance) 1) _refgameinstance))
    (`KismetSystemLibrary.PrintString` (`KismetStringLibrary.Concat_StrStr` "The number f deaths in total are " (`KismetStringLibrary.Conv_IntToString` _output_get)))))

(fn `UserConstructionScript`)