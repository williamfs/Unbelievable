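; BP_LoadNextLevel is an overlap-triggered actor that moves the player on to the next level.
; When the player pawn overlaps it, it adds the game mode's TransitionFade widget to the viewport, waits briefly, then calls LoadNextLevel on BP_GameInstance.
; A disconnected leftover chain would show the mouse cursor and a ThanksForPlaying screen, but it never runs.
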(event `self.ReceiveActorBeginOverlap`
  (params (OtherActor :type "Actor Object Reference"))
  ;[1 1 1] Increase and Load Next Level
  (if (== OtherActor (`GameplayStatics.GetPlayerPawn` 0))
    (`UserWidget.AddToViewport` (`/Game/Blueprints/BP_GameMode.TransitionFade` (cast `/Game/Blueprints/BP_GameMode` (`GameplayStatics.GetGameMode`) :!pure true)) 0)
    (`KismetSystemLibrary.Delay` 1.0)
    (`/Game/Blueprints/BP_GameInstance.LoadNextLevel` (cast `/Game/Blueprints/BP_GameInstance` (`GameplayStatics.GetGameInstance`) :!pure true))))

(fn `UserConstructionScript`)