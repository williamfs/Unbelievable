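; Platform actor whose material and collision respond to FinalResultNeeded while the player is within a scalable sphere range.
; Timelines blend the material's "Yeeter" parameter toward that value on entering the sphere and back to 1.0 on leaving.
; While in range, Tick applies the value and toggles collision using separate on/off thresholds; standing in the PlayerOnPlatform trigger suspends this.
; Tick also stores the player-to-platform look-at rotation, but FinalResultNeeded's calculation is not in these graphs.
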(event `self.ReceiveBeginPlay`
  (bind _platform (`self.Platform`))
  (set `self.platformRotation` (`SceneComponent.K2_GetComponentRotation` (`self.DefaultSceneRoot`)))
  (`PrimitiveComponent.SetMaterial` _platform 0 "/Game/Geometry/Platforms/Materials/M_Platform_Peripheral.M_Platform_Peripheral")
  (bind _returnvalue (`PrimitiveComponent.CreateDynamicMaterialInstance` _platform 0 "/Game/Geometry/Platforms/Materials/M_Platform_Peripheral.M_Platform_Peripheral" "None"))
  (set `self.REFMaterial` _returnvalue)
  (`SceneComponent.SetWorldScale3D` (`self.Sphere`) (`self.PeripheralRange`)))

(event `self.ReceiveTick`
  (params (DeltaSeconds :type "Float (single-precision)"))
  (bind _platform (`self.Platform`))
  (set `self.platformRotation` (`KismetMathLibrary.FindLookAtRotation` (`SceneComponent.K2_GetComponentLocation` (`Actor.RootComponent` (`GameplayStatics.GetPlayerPawn` 0))) (`SceneComponent.K2_GetComponentLocation` (`self.DefaultSceneRoot`))))
  (if (`self.isPlayerInRange`)
    (`MaterialInstanceDynamic.SetScalarParameterValue` (`self.REFMaterial`) "Yeeter" (`self.finalResultNeeded`))
    (if (>= (`self.finalResultNeeded`) 0.75)
      (`PrimitiveComponent.SetCollisionEnabled` _platform "QueryAndPhysics")
      (elif (<= (`self.finalResultNeeded`) 0.3)
        (`PrimitiveComponent.SetCollisionEnabled` _platform "NoCollision")))))

(event `self.Sphere.OnComponentBeginOverlap`
  (params (OverlappedComponent :type "PrimitiveComponent Object Reference") (OtherActor :type "Actor Object Reference") (OtherComp :type "PrimitiveComponent Object Reference") (OtherBodyIndex :type Integer) (bFromSweep :type Boolean) (SweepResult :type "HitResult Structure (by ref)"))
  (if (== OtherActor (`GameplayStatics.GetPlayerPawn` 0))
    (bind _returnvalue (`MaterialInstanceDynamic.K2_GetScalarParameterValue` (`self.REFMaterial`) "Yeeter"))
    (set `self.REFScalarParameter` _returnvalue)
    (bind (_direction _newtrack_0) (`Timeline|LerpEnter` :!via `PlayFromStart`)
      (:`Update`
        (`MaterialInstanceDynamic.SetScalarParameterValue` (`self.REFMaterial`) "Yeeter" (`KismetMathLibrary.Lerp` (`self.REFScalarParameter`) (`self.finalResultNeeded`) _newtrack_0)))
      (:`Finished`
        (set `self.isPlayerInRange` true)))))

(event `self.Sphere.OnComponentEndOverlap`
  (params (OverlappedComponent :type "PrimitiveComponent Object Reference") (OtherActor :type "Actor Object Reference") (OtherComp :type "PrimitiveComponent Object Reference") (OtherBodyIndex :type Integer))
  (if (== OtherActor (`GameplayStatics.GetPlayerPawn` 0))
    (bind _returnvalue (`MaterialInstanceDynamic.K2_GetScalarParameterValue` (`self.REFMaterial`) "Yeeter"))
    (set `self.REFScalarParameter` _returnvalue)
    (bind (_direction _newtrack_0) (`Timeline|LerpExit` :!via `PlayFromStart`)
      (:`Update`
        (`MaterialInstanceDynamic.SetScalarParameterValue` (`self.REFMaterial`) "Yeeter" (`KismetMathLibrary.Lerp` (`self.REFScalarParameter`) 1.0 _newtrack_0)))
      (:`Finished`
        (set `self.isPlayerInRange` false)))))

(event `self.PlayerOnPlatform.OnComponentBeginOverlap`
  (params (OverlappedComponent :type "PrimitiveComponent Object Reference") (OtherActor :type "Actor Object Reference") (OtherComp :type "PrimitiveComponent Object Reference") (OtherBodyIndex :type Integer) (bFromSweep :type Boolean) (SweepResult :type "HitResult Structure (by ref)"))
  (if (== OtherActor (`GameplayStatics.GetPlayerPawn` 0))
    (set `self.isPlayerInRange` false)))

(event `self.PlayerOnPlatform.OnComponentEndOverlap`
  (params (OverlappedComponent :type "PrimitiveComponent Object Reference") (OtherActor :type "Actor Object Reference") (OtherComp :type "PrimitiveComponent Object Reference") (OtherBodyIndex :type Integer))
  (if (== OtherActor (`GameplayStatics.GetPlayerPawn` 0))
    (set `self.isPlayerInRange` true)))

(fn `UserConstructionScript`)