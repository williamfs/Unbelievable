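; BP_BendyTree is an actor with left and right tree components that rotate according to the player pawn's distance from its CenterPoint.
; BeginPlay caches each tree's starting world rotation.
; While IsInRange is true, Tick maps that distance to a clamped alpha, blending both trees from zero world rotation up close back to their starting rotations farther away.
; Nothing shown sets IsInRange.
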(event `self.ReceiveBeginPlay`
  (set `self.REFBendyTreeRRot` (`SceneComponent.K2_GetComponentRotation` (`self.BendyTreeR`)))
  (set `self.REFBendyTreeLRot` (`SceneComponent.K2_GetComponentRotation` (`self.BendyTreeL`))))

(event `self.ReceiveTick`
  (params (DeltaSeconds :type "Float (single-precision)"))
  (bind _returnvalue (`KismetMathLibrary.FClamp` (`KismetMathLibrary.NormalizeToRange` (`KismetMathLibrary.VSize` (- (`SceneComponent.K2_GetComponentLocation` (`self.CenterPoint`)) (`self.K2_GetActorLocation` (`GameplayStatics.GetPlayerPawn` 0)))) 1.0 700.0)))
  (if (`self.isInRange`)
    (`SceneComponent.K2_SetWorldRotation` (`self.BendyTreeR`) (`KismetMathLibrary.RLerp` (struct) (`self.REFBendyTreeRRot`) _returnvalue) false false)
    (`SceneComponent.K2_SetWorldRotation` (`self.BendyTreeL`) (`KismetMathLibrary.RLerp` (struct) (`self.REFBendyTreeLRot`) _returnvalue) false false)))

(fn `UserConstructionScript`)