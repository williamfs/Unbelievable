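; BP_Projectile is a homing projectile that targets the player's capsule and destroys itself after a set lifespan.
; On sphere overlap it takes one health point from the player and destroys itself, without checking what it hit.
; The overlap switch, marked temporary, runs on a fixed value, so its player-death branch never runs and the game instance's selected mode is unused.
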(event `self.ReceiveBeginPlay`
  (bind _asfirst_person_character (cast `/Game/FirstPersonCPP/Blueprints/FirstPersonCharacter` (`GameplayStatics.GetPlayerPawn` 0) :!pure true))
  ;[1 1 1] Set Refs and Proj Lifespan
  (bind _asbp_game_instance (cast `/Game/Blueprints/BP_GameInstance` (`GameplayStatics.GetGameInstance`)))
  (set `self.ref_GameInstance` _asbp_game_instance)
  (set `ProjectileMovementComponent.HomingTargetComponent` (`Character.CapsuleComponent` _asfirst_person_character) (`self.ProjectileMovement`))
  (set `self.REFPlayerCharacter` _asfirst_person_character)
  (`KismetSystemLibrary.Delay` (`self.ProjectileLifespan`))
  (`self.K2_DestroyActor`))

(event `self.Sphere.OnComponentBeginOverlap`
  (params (OverlappedComponent :type "PrimitiveComponent Object Reference") (OtherActor :type "Actor Object Reference") (OtherComp :type "PrimitiveComponent Object Reference") (OtherBodyIndex :type Integer) (bFromSweep :type Boolean) (SweepResult :type "HitResult Structure (by ref)"))
  (bind _refplayercharacter (`self.REFPlayerCharacter`))
  ;[1 1 1] Temp Projectile Functionality
  (switch `int` 2
    (:`2`
      (set `UnbelievableCharacter.healthPoints` (- (`UnbelievableCharacter.healthPoints` _refplayercharacter) 1) _refplayercharacter :!label _label)
      (`self.K2_DestroyActor`))
    (:`3`
      (goto _label))
    (:`4`
      (if (== OtherActor (`GameplayStatics.GetPlayerPawn` 0))
        (`/Game/Blueprints/BP_GameMode.PlayerDeath` (cast `/Game/Blueprints/BP_GameMode` (`GameplayStatics.GetGameMode`) :!pure true))
        (`self.K2_DestroyActor`)))))

(fn `UserConstructionScript`)