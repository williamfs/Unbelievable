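; Game mode for a first-person game that handles player death and respawn and holds the fade and end-screen widgets.
; BeginPlay creates the death fade, thanks-for-playing and transition widgets; FadeIn displays the death fade.
; PlayerDeath stops the character, teleports it to SpawnLocation, resets tagged breaking platforms and destroys all projectiles.
; Shake is disabled on death and re-enabled through a delayed event called only from the BP_BreakingPlatform2 reset branch.
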(event `self.ReceiveBeginPlay`
  (bind _returnvalue (`GameplayStatics.GetPlayerController` 0))
  (bind _returnvalue_2 (`|CreateWidget` "/Game/Widgets/W_DeathFade.W_DeathFade_C" _returnvalue))
  (set `self.DeathFade` _returnvalue_2)
  (bind _returnvalue_3 (`|CreateWidget` "/Game/Widgets/Thanks_for_Playing.Thanks_for_Playing_C" _returnvalue))
  (set `self.ThanksForPlaying` _returnvalue_3)
  (bind _returnvalue_4 (`|CreateWidget` "/Game/Widgets/W_TransitionFadeOut.W_TransitionFadeOut_C" _returnvalue))
  (set `self.TransitionFade` _returnvalue_4))

(event `WaitToShake`
  (`KismetSystemLibrary.Delay` 1.0)
  (set `UnbelievableCharacter.shouldShake` true (cast `/Game/FirstPersonCPP/Blueprints/FirstPersonCharacter` (`GameplayStatics.GetPlayerPawn` 0) :!pure true)))

(fn `FadeIn`
  (`UserWidget.AddToViewport` (`self.DeathFade`) 0))

(fn `PlayerDeath`
  (bind (_spawnlocation_location _spawnlocation_rotation) (`KismetMathLibrary.BreakTransform` (`self.SpawnLocation`)))
  (bind _asfirst_person_character (cast `/Game/FirstPersonCPP/Blueprints/FirstPersonCharacter` (`GameplayStatics.GetPlayerPawn` 0) :!pure true))
  (set `UnbelievableCharacter.shouldShake` false _asfirst_person_character)
  (set `MovementComponent.Velocity` (0.0 0.0 0.0) (`Character.CharacterMovement` _asfirst_person_character))
  (`self.K2_SetActorLocation` _asfirst_person_character _spawnlocation_location false false)
  (`Controller.SetControlRotation` (`GameplayStatics.GetPlayerController` 0) _spawnlocation_rotation)
  ;[1 1 1] Reset Breaking Platforms
  (bind _outactors (`GameplayStatics.GetAllActorsWithTag` "BreakingPlatform"))
  (for _array_element _outactors
    (bind _asbp_breaking_platform (cast `/Game/Blueprints/Platforms/BP_BreakingPlatform` _array_element)
      (:`then`
        (`/Game/Blueprints/Platforms/BP_BreakingPlatform.ResetPos` _asbp_breaking_platform))
      (:`CastFailed`
        _))
    (bind _asbp_breaking_platform_2 (cast `/Game/Blueprints/Platforms/BP_BreakingPlatform2` _array_element))
    (`/Game/Blueprints/Platforms/BP_BreakingPlatform2.ResetPos` _asbp_breaking_platform_2)
    (`self.WaitToShake`))
  (bind _outactors_2 (`GameplayStatics.GetAllActorsOfClass` "/Game/Blueprints/BP_Projectile.BP_Projectile_C"))
  (for _array_element_2 _outactors_2
    (`self.K2_DestroyActor` _array_element_2)))

(fn `UserConstructionScript`)