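; BP_PortalFlipped is a turret actor that turns toward the player and fires projectiles while the player is inside its cone trigger.
; Cone overlap toggles tracking on Tick and starts or clears a looping fire timer at the RateOfFire interval.
; Each shot spawns BP_Projectile only if a line trace from the spawn point hits the player first.
; When the player leaves, a timeline eases it back to its starting rotation.
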(event `self.ReceiveBeginPlay`
  ;[1 1 1] Set Refs
  (set `self.REFPlayerCharacter` (cast `/Game/FirstPersonCPP/Blueprints/FirstPersonCharacter` (`GameplayStatics.GetPlayerPawn` 0) :!pure true))
  (set `self.REFOriginalRot` (`self.K2_GetActorRotation`))
  (`SceneComponent.SetWorldScale3D` (`self.Cone`) (`self.ConeRadius`)))

(event `self.ReceiveTick`
  (params (DeltaSeconds :type "Float (single-precision)"))
  ;[1 1 1] Look at player when in range
  (if (`self.PlayerInRange`)
    (`self.K2_SetActorRotation` (`KismetMathLibrary.RLerp` (`self.K2_GetActorRotation`) (`KismetMathLibrary.FindLookAtRotation` (`SceneComponent.K2_GetComponentLocation` (`self.DefaultSceneRoot`)) (`self.K2_GetActorLocation` (`GameplayStatics.GetPlayerPawn` 0))) (* DeltaSeconds 50.0)))))

(event `self.Cone.OnComponentBeginOverlap`
  (params (OverlappedComponent :type "PrimitiveComponent Object Reference") (OtherActor :type "Actor Object Reference") (OtherComp :type "PrimitiveComponent Object Reference") (OtherBodyIndex :type Integer) (bFromSweep :type Boolean) (SweepResult :type "HitResult Structure (by ref)"))
  ;[1 1 1] Follow Bool Set
  (if (== OtherActor (`GameplayStatics.GetPlayerPawn` 0))
    (set `self.PlayerInRange` true)
    (`KismetSystemLibrary.K2_SetTimer` null "ShootAtPlayer" (`self.RateOfFire`) true)))

(event `self.Cone.OnComponentEndOverlap`
  (params (OverlappedComponent :type "PrimitiveComponent Object Reference") (OtherActor :type "Actor Object Reference") (OtherComp :type "PrimitiveComponent Object Reference") (OtherBodyIndex :type Integer))
  ;[1 1 1] Follow Bool Set
  (if (== OtherActor (`GameplayStatics.GetPlayerPawn` 0))
    (set `self.PlayerInRange` false)
    (`KismetSystemLibrary.K2_ClearTimer` null "ShootAtPlayer")
    (`self.ResetPos`)))

(event `ShootAtPlayer`
  ;[1 1 1] Looped Fire Function
  (if (`self.PlayerInRange`)
    (`self.TurretFire`)))

(event `ResetPos`
  ;[1 1 1] Reset Rotation
  (bind (_direction _newtrack_0) (`Timeline|ResetTimeline` :!via `PlayFromStart`)
    (:`Update`
      (`self.K2_SetActorRotation` (`KismetMathLibrary.RLerp` (`self.K2_GetActorRotation`) (`self.REFOriginalRot`) _newtrack_0)))))

(fn `TurretFire`
  ;[1 1 1] Trace for Player
  (bind _outhit (`KismetSystemLibrary.LineTraceSingleForObjects` (`SceneComponent.K2_GetComponentLocation` (`self.ProjectileSpawnPoint`)) (`self.K2_GetActorLocation` (`self.REFPlayerCharacter`)) (`|MakeArray` "ObjectTypeQuery1" "ObjectTypeQuery3" :!type "EObjectTypeQuery Enum")))
  (bind (_bblockinghit _binitialoverlap _time _distance _location _impactpoint _normal _impactnormal _physmat _hitactor) (`GameplayStatics.BreakHitResult` _outhit))
  (if (and _bblockinghit (== _hitactor (`self.REFPlayerCharacter`)))
    (`|SpawnActorFromClass` "/Game/Blueprints/BP_Projectile.BP_Projectile_C" (`SceneComponent.K2_GetComponentToWorld` (`self.ProjectileSpawnPoint`)) "Undefined" "OverrideRootScale" null (0.0 0.0 0.0) null)))

(fn `UserConstructionScript`)