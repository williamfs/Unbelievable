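; BP_DodgeSetup is a sliding fence gate that opens when the player pawn enters its Box trigger and closes when it leaves.
; BeginPlay caches the fence's start location, then two timelines ease it toward a fixed diagonal world offset or back, lerping from its current position each update.
; Any overlap begin or end stops the opposing timeline before the player check.
; GateClosing is set on exit but never read here.
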(event `self.ReceiveBeginPlay`
  (set `self.REFStartingLoc` (`SceneComponent.K2_GetComponentLocation` (`self.Fence`))))

(event `GateRollOut`
  (bind (_direction _newtrack_0) (`Timeline|Timeline_0` :!via `PlayFromStart` :!label _label)
    (:`Update`
      (`SceneComponent.K2_SetWorldLocation` (`self.Fence`) (`KismetMathLibrary.VLerp` (`SceneComponent.K2_GetComponentLocation` (`self.Fence`)) (+ (`self.REFStartingLoc`) (-185.0 -185.0 0.0)) (* _newtrack_0 0.2)) false false))))

(event `StopRollOut`
  (goto _label :!via `Stop`))

(event `GateRollIn`
  (bind (_direction _newtrack_0) (`Timeline|Timeline_1` :!via `PlayFromStart` :!label _label_2)
    (:`Update`
      (`SceneComponent.K2_SetWorldLocation` (`self.Fence`) (`KismetMathLibrary.VLerp` (`SceneComponent.K2_GetComponentLocation` (`self.Fence`)) (`self.REFStartingLoc`) (* _newtrack_0 0.2)) false false))))

(event `StopRollIn`
  (goto _label_2 :!via `Stop`))

(event `self.Box.OnComponentBeginOverlap`
  (params (OverlappedComponent :type "PrimitiveComponent Object Reference") (OtherActor :type "Actor Object Reference") (OtherComp :type "PrimitiveComponent Object Reference") (OtherBodyIndex :type Integer) (bFromSweep :type Boolean) (SweepResult :type "HitResult Structure (by ref)"))
  (`self.StopRollIn`)
  (if (== OtherActor (`GameplayStatics.GetPlayerPawn` 0))
    (`self.GateRollOut`)))

(event `self.Box.OnComponentEndOverlap`
  (params (OverlappedComponent :type "PrimitiveComponent Object Reference") (OtherActor :type "Actor Object Reference") (OtherComp :type "PrimitiveComponent Object Reference") (OtherBodyIndex :type Integer))
  (`self.StopRollOut`)
  (if (== OtherActor (`GameplayStatics.GetPlayerPawn` 0))
    (set `self.GateClosing` true)
    (`self.GateRollIn`)))

(fn `UserConstructionScript`)