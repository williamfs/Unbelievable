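; BP_FloatingLight is an actor that bobs endlessly up and down between its placed location and a point 55 units below it.
; BeginPlay caches both endpoints, then waits a random delay of up to two seconds so multiple instances move out of sync.
; Hover and HoverReverse each drive a timeline that lerps the actor location, calling each other on finish to form the loop.
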(event `self.ReceiveBeginPlay`
  (bind _output_get (set `self.REFOriginalLoc` (`self.K2_GetActorLocation`)))
  (set `self.REFHoverDestination` (- _output_get (0.0 0.0 55.0)))
  (`KismetSystemLibrary.Delay` (`KismetMathLibrary.RandomFloatInRange` 0.0 2.0))
  (`self.Hover`))

(event `Hover`
  (bind (_direction _floatlerp) (`Timeline|Timeline_0` :!via `PlayFromStart`)
    (:`Update`
      (`self.K2_SetActorLocation` (`KismetMathLibrary.VLerp` (`self.REFOriginalLoc`) (`self.REFHoverDestination`) _floatlerp)))
    (:`Finished`
      (`self.HoverReverse`))))

(event `HoverReverse`
  (bind (_direction _floatlerp) (`Timeline|Timeline_1` :!via `PlayFromStart`)
    (:`Update`
      (`self.K2_SetActorLocation` (`KismetMathLibrary.VLerp` (`self.REFHoverDestination`) (`self.REFOriginalLoc`) _floatlerp)))
    (:`Finished`
      (`self.Hover`))))

(fn `UserConstructionScript`)