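; A breaking platform Blueprint that moves away from its position when the player enters its trigger.
; The BreakOverlap trigger plays the Break timeline, whose tracks drive a lerped offset from the current actor location, intended as a rumble and fall.
; Tick constantly applies small random rotation jitter to the Platform component.
; ResetPos restores the transform cached at BeginPlay, intended for player death; Shake is empty.
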(event `self.ReceiveTick`
  (params (DeltaSeconds :type "Float (single-precision)"))
  ;[1 1 1] Set Loc Ref
  (`SceneComponent.K2_AddLocalRotation` (`self.Platform`) (`KismetMathLibrary.MakeRotator` (`KismetMathLibrary.RandomFloatInRange` -0.2 0.2) (`KismetMathLibrary.RandomFloatInRange` -0.2 0.2) (`KismetMathLibrary.RandomFloatInRange` -0.2 0.2)) false false))

(event `self.ReceiveBeginPlay`
  ;[1 1 1] Set Loc Ref
  (set `self.REFTransform` (`self.GetTransform`)))

(event `Shake`
  ;[1 1 1] Set Loc Ref
)

(event `self.BreakOverlap.OnComponentBeginOverlap`
  (params (OverlappedComponent :type "PrimitiveComponent Object Reference") (OtherActor :type "Actor Object Reference") (OtherComp :type "PrimitiveComponent Object Reference") (OtherBodyIndex :type Integer) (bFromSweep :type Boolean) (SweepResult :type "HitResult Structure (by ref)"))
  (bind _returnvalue (`self.K2_GetActorLocation`))
  ;[1 1 1] Rumble and Fall
  (if (== OtherActor (`GameplayStatics.GetPlayerPawn` 0))
    (bind (_direction _newtrack_0 _newtrack_1) (`Timeline|Break` :!via `PlayFromStart`)
      (:`Update`
        (`self.K2_SetActorLocation` (`KismetMathLibrary.VLerp` _returnvalue (+ _returnvalue _newtrack_1) _newtrack_0))))))

(event `ResetPos`
  (bind (_reftransform_location _reftransform_rotation) (`KismetMathLibrary.BreakTransform` (`self.REFTransform`)))
  ;[1 1 1] Reset On Player Death
  (`self.K2_SetActorLocationAndRotation` _reftransform_location _reftransform_rotation))

(fn `UserConstructionScript`)