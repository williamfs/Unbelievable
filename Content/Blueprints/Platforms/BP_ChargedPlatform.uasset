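; BP_ChargedPlatform is a bounce pad that launches the player character straight upward on overlap.
; On BeginPlay it creates a dynamic emissive material and loops an idle pulse timeline that drives the Emission parameter.
; A player overlap stops the idle pulse and plays a bounce pulse timeline on the same parameter, which restarts the idle loop when it finishes.
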(event `BouncePulse`
  (`self.IdlePause`)
  (bind (_direction _newtrack_0) (`Timeline|BouncePulseTimeline` :!via `PlayFromStart`)
    (:`Update`
      (`MaterialInstanceDynamic.SetScalarParameterValue` (`self.REFMaterial`) "Emission" _newtrack_0))
    (:`Finished`
      (`self.IdlePulse`))))

(event `IdlePulse`
  (bind (_direction _pulse) (`Timeline|PulseTimeline` :!via `PlayFromStart` :!label _label)
    (:`Update`
      (`MaterialInstanceDynamic.SetScalarParameterValue` (`self.REFMaterial`) "Emission" _pulse))
    (:`Finished`
      (`self.IdlePulse`))))

(event `IdlePause`
  (goto _label :!via `Stop`))

(event `self.ReceiveBeginPlay`
  (bind _platform (`self.Platform`))
  (`PrimitiveComponent.SetMaterial` _platform 0 "/Game/Geometry/Platforms/Materials/M_PlatformCone_Emissive.M_PlatformCone_Emissive")
  (bind _returnvalue (`PrimitiveComponent.CreateDynamicMaterialInstance` _platform 0 "/Game/Geometry/Platforms/Materials/M_PlatformCone_Emissive.M_PlatformCone_Emissive" "None"))
  (set `self.REFMaterial` _returnvalue)
  (`self.IdlePulse`))

(event `self.ReceiveActorBeginOverlap`
  (params (OtherActor :type "Actor Object Reference"))
  (if (== OtherActor (`GameplayStatics.GetPlayerPawn` 0))
    (`Character.LaunchCharacter` (`GameplayStatics.GetPlayerCharacter` 0) (0.0 0.0 2000.0) false false)
    (`self.BouncePulse`)))

(fn `UserConstructionScript`)