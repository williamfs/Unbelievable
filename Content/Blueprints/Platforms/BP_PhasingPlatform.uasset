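; Platform Blueprint for a rock that repeatedly blinks, becomes non-solid, then returns.
; After a random start delay, PhasingOut calls itself on short delays, toggling visibility with a FlipFlop until TimesBlinked matches TimesToBlink, then disables collision.
; PhasingIn waits, restores visibility and collision, resets the counter and restarts the cycle after a pause.
; Disconnected material and Timeline nodes never run.
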(event `self.ReceiveBeginPlay`
  (`KismetSystemLibrary.Delay` (`KismetMathLibrary.RandomFloatInRange` 1.0 3.0))
  (`self.PhasingOut`))

(event `PhasingOut`
  (bind _rock (`self.Rock`))
  (`KismetSystemLibrary.Delay` 0.2)
  (`/Engine/EditorBlueprintResources/StandardMacros.IncrementInt` (`self.TimesBlinked`)
    (:`  `
      (`/Engine/EditorBlueprintResources/StandardMacros.FlipFlop`
        (:`A`
          (`SceneComponent.SetVisibility` _rock false false))
        (:`B`
          (`SceneComponent.SetVisibility` _rock true false)))
      (if (== (`self.TimesBlinked`) (`self.TimesToBlink`))
        (`PrimitiveComponent.SetCollisionEnabled` _rock "NoCollision")
        (`self.PhasingIn`)
        (else
          (`self.PhasingOut`))))))

(event `PhasingIn`
  (bind _rock (`self.Rock`))
  (`KismetSystemLibrary.Delay` 2.0)
  (`SceneComponent.SetVisibility` _rock true false)
  (`PrimitiveComponent.SetCollisionEnabled` _rock "QueryAndPhysics")
  (set `self.TimesBlinked` 1)
  (`KismetSystemLibrary.Delay` 5.0)
  (`self.PhasingOut`))

(fn `UserConstructionScript`)