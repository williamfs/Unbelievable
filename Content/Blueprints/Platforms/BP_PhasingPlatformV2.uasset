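; Phasing rock platform Blueprint, apparently an unfinished rework that moves from blinking to a material opacity fade.
; BeginPlay assigns the phasing material to Rock, then after a delay creates a dynamic instance and plays a timeline driving its Opacity, with debug prints.
; That instance is never assigned to Rock.
; The older blink, collision-toggle and random-start logic is disconnected, leaving PhasingIn and PhasingOut empty.
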(event `self.ReceiveBeginPlay`
  (`PrimitiveComponent.SetMaterial` (`self.Rock`) 0 "/Game/Geometry/Platforms/Materials/M_Platform_Phasing.M_Platform_Phasing")
  (`KismetSystemLibrary.Delay` 2.0)
  (bind _returnvalue (`KismetMaterialLibrary.CreateDynamicMaterialInstance` "/Game/Geometry/Platforms/Materials/M_Platform_Phasing.M_Platform_Phasing"))
  (bind (_direction _newtrack_0) (`Timeline|Timeline_0` :!via `PlayFromStart`)
    (:`Update`
      (`KismetSystemLibrary.PrintString` (`KismetStringLibrary.Conv_DoubleToString` _newtrack_0))
      (`MaterialInstanceDynamic.SetScalarParameterValue` _returnvalue "Opacity" _newtrack_0))
    (:`Finished`
      (`KismetSystemLibrary.PrintString` "Done"))))

(event `PhasingOut`)

(event `PhasingIn`)

(fn `UserConstructionScript`)