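; BP_PeripheralPlatform is a rock platform that fades in and out, with collision disabled when it turns invisible and restored when it turns visible.
; A dynamic material instance created at BeginPlay has its "Yeeter" scalar driven by one timeline per direction, each guarded by a flag.
; Collision switches as each fade starts, and separate stop events halt a fade and save the current scalar value.
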(event `self.ReceiveBeginPlay`
  (bind _rock (`self.Rock`))
  (`PrimitiveComponent.SetMaterial` _rock 0 "/Game/Geometry/Platforms/Materials/M_Platform_Peripheral.M_Platform_Peripheral")
  (bind _returnvalue (`PrimitiveComponent.CreateDynamicMaterialInstance` _rock 0 "/Game/Geometry/Platforms/Materials/M_Platform_Peripheral.M_Platform_Peripheral" "None"))
  (set `self.REFPeripheralPlatform` _returnvalue))

(event `BecomeInvisible`
  (if (not (`self.IsFading`))
    (set `self.IsFading` true)
    (`PrimitiveComponent.SetCollisionEnabled` (`self.Rock`) "NoCollision")
    (bind (_direction _newtrack_0) (`Timeline|Timeline_0` :`NewTime` (`self.curParamaterValue`) :!via `PlayFromStart` :!label _label)
      (:`Update`
        (`MaterialInstanceDynamic.SetScalarParameterValue` (`self.REFPeripheralPlatform`) "Yeeter" _newtrack_0))
      (:`Finished`
        (set `self.IsFading` false)))))

(event `StopFadeOut`
  (bind _returnvalue (`MaterialInstanceDynamic.K2_GetScalarParameterValue` (`self.REFPeripheralPlatform`) "Yeeter"))
  (set `self.curParamaterValue` _returnvalue)
  (set `self.IsFading` false)
  (goto _label :!via `Stop`))

(event `BecomeVisible`
  (if (not (`self.IsBecomingVisible`))
    (set `self.IsBecomingVisible` true)
    (`PrimitiveComponent.SetCollisionEnabled` (`self.Rock`) "QueryAndPhysics")
    (bind (_direction _newtrack_0) (`Timeline|Timeline_1` :`NewTime` (`self.curParamaterValue`) :!via `PlayFromStart` :!label _label_2)
      (:`Update`
        (`MaterialInstanceDynamic.SetScalarParameterValue` (`self.REFPeripheralPlatform`) "Yeeter" _newtrack_0))
      (:`Finished`
        (set `self.IsBecomingVisible` false)))))

(event `StopFadeIn`
  (bind _returnvalue (`MaterialInstanceDynamic.K2_GetScalarParameterValue` (`self.REFPeripheralPlatform`) "Yeeter"))
  (set `self.curParamaterValue` _returnvalue)
  (set `self.IsBecomingVisible` false)
  (goto _label_2 :!via `Stop`))

(fn `UserConstructionScript`)