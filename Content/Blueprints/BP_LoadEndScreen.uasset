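; BP_LoadEndScreen is a trigger actor that shows the end-of-game screen when the player pawn overlaps it.
; On overlap it adds the game mode's TransitionFade widget to the viewport, waits briefly, then enables the mouse cursor and adds the ThanksForPlaying widget.
; A LoadNextLevel call on the game instance remains in the graph but never runs.
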(event `self.ReceiveActorBeginOverlap`
  (params (OtherActor :type "Actor Object Reference"))
  (bind _asbp_game_mode (cast `/Game/Blueprints/BP_GameMode` (`GameplayStatics.GetGameMode`) :!pure true))
  ;[1 1 1] Increase and Load Next Level
  (if (== OtherActor (`GameplayStatics.GetPlayerPawn` 0))
    (`UserWidget.AddToViewport` (`/Game/Blueprints/BP_GameMode.TransitionFade` _asbp_game_mode) 0)
    (`KismetSystemLibrary.Delay` 0.6)
    (set `PlayerController.bShowMouseCursor` true (`GameplayStatics.GetPlayerController` 0))
    (`UserWidget.AddToViewport` (`/Game/Blueprints/BP_GameMode.ThanksForPlaying` _asbp_game_mode) 0)))

(fn `UserConstructionScript`)