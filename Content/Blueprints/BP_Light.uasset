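; BP_Light is a collectible light orb that the player picks up by overlapping its PickupVolume.
; On BeginPlay it creates a dynamic emissive material instance for the Orb mesh.
; The first player overlap calls OrbCollectionRim on BP_GameMode, then a timeline drives the material's Fade parameter and destroys the actor when it finishes.
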(event `self.ReceiveBeginPlay`
  (bind _returnvalue (`PrimitiveComponent.CreateDynamicMaterialInstance` (`self.Orb`) 0 "/Game/Particles/M_EmissiveLight.M_EmissiveLight" "None")))

(event `self.PickupVolume.OnComponentBeginOverlap`
  (params (OverlappedComponent :type "PrimitiveComponent Object Reference") (OtherActor :type "Actor Object Reference") (OtherComp :type "PrimitiveComponent Object Reference") (OtherBodyIndex :type Integer) (bFromSweep :type Boolean) (SweepResult :type "HitResult Structure (by ref)"))
  (if (== OtherActor (`GameplayStatics.GetPlayerPawn` 0))
    (`/Engine/EditorBlueprintResources/StandardMacros.DoOnce` false
      (:`Completed`
        (`/Game/Blueprints/BP_GameMode.OrbCollectionRim` (cast `/Game/Blueprints/BP_GameMode` (`GameplayStatics.GetGameMode`) :!pure true))
        (bind (_direction _newtrack_0) (`Timeline|LerpFade` :!via `PlayFromStart`)
          (:`Update`
            (`MaterialInstanceDynamic.SetScalarParameterValue` (stale `self.ReceiveBeginPlay` _returnvalue) "Fade" _newtrack_0))
          (:`Finished`
            (`self.K2_DestroyActor`)))))))

(fn `UserConstructionScript`)