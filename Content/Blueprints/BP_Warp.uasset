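; BP_Warp is a teleporter actor that moves the player pawn to a linked Destination actor.
; Overlapping its Box relocates the pawn and zeroes its movement velocity, provided the PlayerCanTeleport flag on BP_GameMode is set.
; It clears that shared flag during the warp, then restores it through WaitToTeleport after TeleportUseDelay as a global cooldown.
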(event `self.Box.OnComponentBeginOverlap`
  (params (OverlappedComponent :type "PrimitiveComponent Object Reference") (OtherActor :type "Actor Object Reference") (OtherComp :type "PrimitiveComponent Object Reference") (OtherBodyIndex :type Integer) (bFromSweep :type Boolean) (SweepResult :type "HitResult Structure (by ref)"))
  (bind _asbp_game_mode (cast `/Game/Blueprints/BP_GameMode` (`GameplayStatics.GetGameMode`) :!pure true))
  ;[1 1 1] Teleport Functionality
  (if (and (== OtherActor (`GameplayStatics.GetPlayerPawn` 0)) (`/Game/Blueprints/BP_GameMode.PlayerCanTeleport` _asbp_game_mode))
    (set `/Game/Blueprints/BP_GameMode.PlayerCanTeleport` false _asbp_game_mode)
    (`self.K2_SetActorLocation` (`GameplayStatics.GetPlayerPawn` 0) (`self.K2_GetActorLocation` (`self.Destination`)) false false)
    (set `MovementComponent.Velocity` (0.0 0.0 0.0) (`Pawn.GetMovementComponent` (`GameplayStatics.GetPlayerPawn` 0)))
    (`KismetSystemLibrary.Delay` (`self.TeleportUseDelay`))
    (`self.WaitToTeleport`)))

(fn `UserConstructionScript`)

(fn `WaitToTeleport`
  (set `/Game/Blueprints/BP_GameMode.PlayerCanTeleport` true (cast `/Game/Blueprints/BP_GameMode` (`GameplayStatics.GetGameMode`) :!pure true)))